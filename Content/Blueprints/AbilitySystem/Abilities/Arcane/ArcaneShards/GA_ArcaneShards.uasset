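; Gameplay Ability for the Arcane Shards spell, which spawns shards at random locations derived from a player-chosen point.
; On activation it shows a magic circle, then waits for an input press to commit, ending if the commit fails.
; The mouse hit point turns the avatar, hides the circle and starts the cast montage.
; A montage gameplay event triggers the shard spawn, and the ability ends shortly after it succeeds.
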(event Ability|EventActivateAbility
  (Utilities|FlowControl|Sequence
    (:then_0
      (Class|PlayerInterface|ShowMagicCircle(Message) (Ability|GetAvatarActorfromActorInfo) 0))
    (:then_1
      (Ability|Tasks|WaitInputPress false
        (:OnPress
          (bind _returnvalue (Ability|CommitAbility))
          (if _returnvalue
            (bind _datahandle (|TargetDataUnderMouse)
              (:ValidData
                (bind _output_get (Variables|Default|SetMouseHitLocation (.impactpoint (Ability|TargetData|GetHitResultfromTargetData _datahandle))))
                (Class|CombatInterface|UpdateFacingTarget(Message) (Ability|GetAvatarActorfromActorInfo) _output_get)
                (Class|PlayerInterface|HideMagicCircle(Message) (Ability|GetAvatarActorfromActorInfo))
                (|PlayMontageandWaitProxy "None" "/Game/Assets/Characters/Aura/Animations/Abilities/AM_Cast_ArcaneShards.AM_Cast_ArcaneShards" 1.0 "None" false 1.0 0.0 false
                  (:then
                    (Ability|Tasks|WaitGameplayEvent "(TagName=\"Event.Montage.ArcaneShards\")" 0 true
                      (:EventReceived
                        (|SpawnArcaneShards (Class|AuraArcaneShardsAbility|GetRandomSpawnLocations (Variables|Default|GetMouseHitLocation))
                          (:OnSuccess
                            (Utilities|FlowControl|Delay 0.2)
                            (Ability|EndAbility)))))))))
            (else
              (Ability|EndAbility))))))))

(event Ability|EventOnEndAbility
  (params (bWasCancelled :type Boolean)))