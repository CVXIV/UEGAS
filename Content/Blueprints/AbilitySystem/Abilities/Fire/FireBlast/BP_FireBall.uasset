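; BP_FireBall is a fire blast projectile actor that flies out and then returns, boomerang style.
; When StartOutgoingTimeline runs on the authority, an Outgoing timeline lerps it from its spawn point to an apex a set distance along its forward vector.
; A Returning timeline then lerps it back, tracking ReturnToActor's live location while valid, and calls OnDestroy on finish.
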(event EventBeginPlay)

(event Collision|EventActorBeginOverlap
  (params (OtherActor :type Actor%20Object%20Reference)))

(event EventTick
  (params (DeltaSeconds :type Float%20%28single-precision%29)))

(event EventStartOutgoingTimeline
  (bind _returnvalue (Transformation|GetActorLocation))
  (Networking|SwitchHasAuthority
    (:Authority
      (bind _output_get (Variables|Default|SetInitLocation _returnvalue))
      (Variables|Default|SetReturnLocation _returnvalue)
      (Variables|Default|SetApexLocation (+ _output_get (* (Transformation|GetActorForwardVector) (Variables|Default|GetTraveDistance))))
      (bind _outgoingtrack (Timeline|Outgoing Play)
        (:Update
          (Transformation|SetActorLocation (Math|Vector|Lerp(Vector) (Variables|Default|GetInitLocation) (Variables|Default|GetApexLocation) _outgoingtrack) false false))
        (:Finished
          (bind _returningtrack (Timeline|Returning Play)
            (:Update
              (bind _returntoactor (Variables|Default|GetReturnToActor)
                (:then
                  (Variables|Default|SetReturnLocation (Transformation|GetActorLocation _returntoactor)))
                (:else
                  _))
              (Transformation|SetActorLocation (Math|Vector|Lerp(Vector) (Variables|Default|GetApexLocation) (Variables|Default|GetReturnLocation) _returningtrack) false false))
            (:Finished
              (Class|AuraProjectile|OnDestroy true))))))))

(fn ConstructionScript)