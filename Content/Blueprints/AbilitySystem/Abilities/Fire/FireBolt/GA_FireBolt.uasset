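; Fire Bolt gameplay ability that casts a projectile at whatever is under the mouse cursor.
; After committing, it gets target data under the mouse, turns the avatar toward the hit point and plays the cast montage.
; The montage's gameplay event triggers the projectile spawn with the hit location, hit actor and weapon attack tag.
; The ability then ends while the montage keeps playing, or ends immediately if the commit fails.
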(event Ability|EventActivateAbility
  (bind _returnvalue (Ability|CommitAbility))
  (if _returnvalue
    (bind _datahandle (|TargetDataUnderMouse)
      (:then
        (Class|CombatInterface|UpdateFacingTarget(Message) (Ability|GetAvatarActorfromActorInfo) (.impactpoint (Ability|TargetData|GetHitResultfromTargetData _datahandle)))
        (|PlayMontageandWaitProxy "None" "/Game/Assets/Characters/Aura/Animations/Abilities/AM_Cast_FireBolt.AM_Cast_FireBolt" 1.0 "None" false 1.0 0.0 false
          (:then
            (Ability|Tasks|WaitGameplayEvent "(TagName=\"Event.Montage.FireBolt\")" 0
              (:EventReceived
                (Class|AuraProjectileSpell|SpawnProjectile (.impactpoint (Ability|TargetData|GetHitResultfromTargetData _datahandle)) (.hitactor (Ability|TargetData|GetHitResultfromTargetData _datahandle)) (GameplayTags|MakeLiteralGameplayTag "(TagName=\"Montage.Attack.Weapon\")"))
                (Ability|EndAbility)))))))
    (else
      (Ability|EndAbility))))

(event Ability|EventOnEndAbility
  (params (bWasCancelled :type Boolean)))