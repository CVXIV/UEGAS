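; Melee attack gameplay ability that turns the avatar toward its combat target and plays a random attack montage.
; A gameplay event matching the montage's tag triggers a small sphere check at that tag's combat socket, excluding the avatar.
; Each live player found receives the ability's default damage effect and a MeleeImpact gameplay cue carrying the montage tag.
; The ability ends when the montage completes.
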(event Ability|EventActivateAbility
  (bind _returnvalue (Ability|GetAvatarActorfromActorInfo))
  (bind _returnvalue_2 (Ability|GetAvatarActorfromActorInfo))
  (bind _returnvalue_3 (Class|EnemyInterface|GetCombatTarget(Message) _returnvalue_2))
  (Class|CombatInterface|UpdateFacingTarget(Message) _returnvalue_2 (Transformation|GetActorLocation _returnvalue_3))
  (bind _returnvalue_4 (Class|CombatInterface|GetAttackMontageRandom(Message) _returnvalue_2))
  (|PlayMontageandWaitProxy "None" (.montage _returnvalue_4) 1.0 "None" true 1.0 0.0 false
    (:then
      (Ability|Tasks|WaitGameplayEvent (.montagetag _returnvalue_4) 0
        (:EventReceived
          (bind _returnvalue_5 (Class|CombatInterface|GetCombatSocketLocation(Message) _returnvalue (.montagetag _returnvalue_4)))
          (bind _returnvalue_6 (Class|AuraAbilitySystemLibrary|GetLivePlayersWithinRadius _returnvalue (Utilities|Array|MakeArray _returnvalue) 45.0 _returnvalue_5))
          (for _array_element _returnvalue_6
            (Class|AuraAbilitySystemLibrary|ApplyGameplayEffect (Class|AuraDamageGameplayAbility|MakeDamageEffectParamsfromClassDefaults (Ability|GetAvatarActorfromActorInfo) _array_element))
            (Class|GameplayAbility|ExecuteGameplayCuewithParams "(TagName=\"GameplayCue.MeleeImpact\")" (Ability|GameplayCue|MakeGameplayCueParameters :AggregatedSourceTags (GameplayTags|MakeGameplayTagContainerfromArray (Utilities|Array|MakeArray (.montagetag _returnvalue_4))) :Location (Transformation|GetActorLocation _array_element) :EffectCauser (Ability|GetAvatarActorfromActorInfo) :SourceObject _array_element))))))
    (:OnCompleted
      (Ability|EndAbility))))

(event Ability|EventOnEndAbility
  (params (bWasCancelled :type Boolean)))