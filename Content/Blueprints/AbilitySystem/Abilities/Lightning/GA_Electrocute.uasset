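; Electrocute gameplay ability that channels an electric beam toward the mouse hit location, dealing damage while input is held.
; On valid mouse target data it hides the cursor, faces the target and plays a montage, whose event starts the shock loop and beam.
; A looping timer pays cost and applies damage each tick.
; Input release or failed cost commit clears the timer, restores the cursor and commits cooldown.
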(event Custom|DamageAndCost
  (bind _returnvalue (Ability|CommitAbilityCost false))
  (if _returnvalue
    (Class|AuraBeamSpell|ApplyDamageOnce)
    (else
      (Class|AuraBeamSpell|OnAbilityEnd))))

(event Ability|EventActivateAbility
  (bind _datahandle (|TargetDataUnderMouse)
    (:ValidData
      (Class|AuraBeamSpell|StoreMouseDataInfo (Ability|TargetData|GetHitResultfromTargetData _datahandle))
      (Class|AuraBeamSpell|StoreOwnerPlayerController)
      (Utilities|FlowControl|Sequence
        (:then_0
          (Variables|/Script/Engine.PlayerController|SetbShowMouseCursor (Variables|Default|GetOwnerPlayerController) false)
          (GameplayCue|ExecuteGameplayCue :GameplayCueTag "(TagName=\"GameplayCue.ShockBurst\")")
          (Class|CombatInterface|UpdateFacingTarget(Message) (Ability|GetAvatarActorfromActorInfo) (Variables|Default|GetMouseHitLocation))
          (|PlayMontageandWaitProxy "None" (Variables|Default|GetMontage_Electrocute) 1.0 "None" false 1.0 0.0 false
            (:then
              (Ability|Tasks|WaitGameplayEvent "(TagName=\"Event.Montage.Electrocute\")" 0 true
                (:EventReceived
                  (Class|CombatInterface|SetinShockLoop(Message) (Ability|GetAvatarActorfromActorInfo) true)
                  (CallFunction|SpawnElectricBeam)
                  (bind _returnvalue (Utilities|Time|SetTimerbyEvent (delegate Custom|DamageAndCost) (Variables|Default|GetDamageDeltaTime) true))
                  (Variables|Default|SetDamageTimer _returnvalue))))))
        (:then_1
          (Ability|Tasks|WaitInputRelease false
            (:OnRelease
              (Class|AuraBeamSpell|OnAbilityEnd))))))))

(event EventOnAbilityEnd
  (|CallParentFunction)
  (Utilities|Time|ClearandInvalidateTimerbyHandle (Variables|Default|GetDamageTimer))
  (Variables|/Script/Engine.PlayerController|SetbShowMouseCursor (Variables|Default|GetOwnerPlayerController) true)
  (Class|CombatInterface|SetinShockLoop(Message) (Ability|GetAvatarActorfromActorInfo) false)
  (Ability|CommitAbilityCooldown false)
  (Ability|EndAbility))

(fn SpawnElectricBeam
  (Class|AuraBeamSpell|TraceFirstTarget (Variables|Default|GetMouseHitLocation))
  (Class|AuraBeamSpell|SpawnElectricBeamwithRange))