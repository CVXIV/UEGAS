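; Flame pillar actor with a flickering point light and the ability to fade out and back in.
; From BeginPlay, a self-restarting loop randomly picks one of two timelines to scale the light's base intensity.
; ActorFadeOut makes the mesh ignore Visibility and a custom trace channel, while a timeline drives the Fade parameter on its dynamic materials.
; ActorFadein restores blocking and reverses that timeline.
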(event Custom|RandomIntensity
  (if (Math|Random|RandomBool)
    (bind _intensity (Timeline|Intensity_1 PlayFromStart)
      (:Update
        (Rendering|Components|Light|SetIntensity (Variables|Default|GetPointLight) (* (Variables|Default|GetBaseIntensity) _intensity)))
      (:Finished
        (CallFunction|RandomIntensity :!label _label)))
    (else
      (bind _intensity_2 (Timeline|Intensity_2 PlayFromStart)
        (:Update
          (Rendering|Components|Light|SetIntensity (Variables|Default|GetPointLight) (* _intensity_2 (Variables|Default|GetBaseIntensity))))
        (:Finished
          (goto _label))))))

(event EventBeginPlay
  (CallFunction|RandomIntensity))

(event Collision|EventActorBeginOverlap
  (params (OtherActor :type Actor%20Object%20Reference)))

(event EventTick
  (params (DeltaSeconds :type Float%20%28single-precision%29)))

(event EventActorFadeOut
  (Collision|SetCollisionResponsetoChannel (Variables|Default|GetStaticMeshComponent) "ECC_GameTraceChannel2" "ECR_Ignore")
  (Collision|SetCollisionResponsetoChannel (Variables|Default|GetStaticMeshComponent) "ECC_Visibility" "ECR_Ignore")
  (bind _fadealpha (Timeline|Fade Play)
    (:Update
      (for _array_element (Variables|Default|GetDynamicInstanceMaterial)
        (Rendering|Material|SetScalarParameterValue _array_element "Fade" _fadealpha :!class /Script/Engine.MaterialInstanceDynamic)))))

(event EventActorFadein
  (Collision|SetCollisionResponsetoChannel (Variables|Default|GetStaticMeshComponent) "ECC_GameTraceChannel2" "ECR_Block")
  (Collision|SetCollisionResponsetoChannel (Variables|Default|GetStaticMeshComponent) "ECC_Visibility" "ECR_Block")
  (bind _fadealpha (Timeline|Fade Reverse)
    (:Update
      (for _array_element (Variables|Default|GetDynamicInstanceMaterial)
        (Rendering|Material|SetScalarParameterValue _array_element "Fade" _fadealpha :!class /Script/Engine.MaterialInstanceDynamic)))))

(fn ConstructionScript)